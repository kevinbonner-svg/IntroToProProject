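; BP_CubeTarget is a physics cube target that awards points when hit and can be returned to its starting position.
; It stores the cube's world transform on BeginPlay, and ResetTargetCube teleports it back, toggling physics simulation off and on around the move.
; HandleHit looks up the first BP_TargetManager in the level and adds a fixed score to it.
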(event `self.ReceiveBeginPlay`
  (set `self.StartLocation` (`SceneComponent.K2_GetComponentToWorld` (`self.Cube`))))

(event `ResetTargetCube`
  (`PrimitiveComponent.SetSimulatePhysics` (`self.Cube`) false)
  (`SceneComponent.K2_SetWorldTransform` (`self.Cube`) (`self.StartLocation`) false true)
  (`PrimitiveComponent.SetSimulatePhysics` (`self.Cube`) true))

(event `/Game/Production/Blueprints/Interfaces/BPI_TargetHit.HandleHit`
  (params (ScoreValue :type Integer))
  (bind _outactors (`GameplayStatics.GetAllActorsOfClass` "/Game/Production/Blueprints/BP_TargetManager.BP_TargetManager_C"))
  (`/Game/Production/Blueprints/BP_TargetManager.AddScore` (`|GetArrayItem` _outactors) 50))

(fn `UserConstructionScript`)