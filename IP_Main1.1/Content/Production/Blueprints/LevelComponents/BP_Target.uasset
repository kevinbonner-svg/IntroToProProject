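; BP_Target is a level target actor with a health component and a sphere mesh.
; It prints the new health as debug text whenever the health component reports a change.
; When health runs out, it prints a death message and calls Reset, which restores maximum health and sets the sphere's material to M_ProjectileBullet, so the target stays in play.
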(event `self.BPC_Health.OnHealthChanged`
  (params (NewHealth :type "Float (double-precision)"))
  (`KismetSystemLibrary.PrintString` (`KismetStringLibrary.Concat_StrStr` "HIT Health" (`KismetStringLibrary.Conv_DoubleToString` NewHealth))))

(event `self.BPC_Health.OnHealthDepleted`
  (`KismetSystemLibrary.PrintString` "TargetDead")
  (`self.Reset`))

(fn `Reset`
  (bind _bpc_health (`self.BPC_Health`))
  (set `/Game/Production/Blueprints/Components/BPC_Health.Health` (`/Game/Production/Blueprints/Components/BPC_Health.MaxHealth` _bpc_health) _bpc_health)
  (`PrimitiveComponent.SetMaterial` (`self.Sphere`) 0 "/Game/Weapons/GrenadeLauncher/Materials/M_ProjectileBullet.M_ProjectileBullet"))

(fn `UserConstructionScript`)