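; A shootable gravity cube level prop that alternates between Idle and Floating states on each shot.
; A shot from Idle disables gravity and launches the cube upward along a Z-only physics constraint; a shot while Floating re-anchors the constraint and locks it in place.
; Angular limits lock at BeginPlay, and ResetTarget restores the saved start transform, gravity and free linear movement.
; HandleHit separately adds score through the first BP_TargetManager found.
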(event `OnShot`
  (bind _physicsconstraint (`self.PhysicsConstraint`))
  (bind _physicsconstraint_2 (`self.PhysicsConstraint`))
  ; Switch between gravity cube states
  (switch `/Game/Production/Blueprints/E_CubeState` (`self.CubeState`)
    (:`NewEnumerator0`
      (`PhysicsConstraintComponent.SetLinearXLimit` _physicsconstraint "LCM_Locked" 0.0)
      (`PhysicsConstraintComponent.SetLinearYLimit` _physicsconstraint "LCM_Locked" 0.0)
      (`PhysicsConstraintComponent.SetLinearZLimit` _physicsconstraint "LCM_Free" 0.0)
      (`PrimitiveComponent.SetEnableGravity` (`self.GravityCube`) false)
      (`PrimitiveComponent.AddImpulse` (`self.GravityCube`) (0.0 0.0 50.0) "None" true)
      (set `self.CubeState` "NewEnumerator1"))
    (:`NewEnumerator1`
      (`SceneComponent.K2_SetWorldLocation` (`self.PhysicsConstraint`) (`SceneComponent.K2_GetComponentLocation` (`self.GravityCube`)) false true)
      (`PhysicsConstraintComponent.SetConstrainedComponents` (`self.PhysicsConstraint`) (`self.GravityCube`) "None" null "None")
      (`PhysicsConstraintComponent.SetLinearXLimit` _physicsconstraint_2 "LCM_Locked" 0.0)
      (`PhysicsConstraintComponent.SetLinearYLimit` _physicsconstraint_2 "LCM_Locked" 0.0)
      (`PhysicsConstraintComponent.SetLinearZLimit` _physicsconstraint_2 "LCM_Locked" 0.0)
      (set `self.CubeState` "NewEnumerator0"))))

(event `self.ReceiveBeginPlay`
  (bind _physicsconstraint (`self.PhysicsConstraint`))
  ; Set Cube Starting Location
  (`|ExecutionSequence`
    (:`then_0`
      (set `self.StartLocation` (`SceneComponent.K2_GetComponentToWorld` (`self.GravityCube`))))
    (:`then_1`
      (`PhysicsConstraintComponent.SetAngularSwing1Limit` _physicsconstraint "ACM_Locked" 0.0)
      (`PhysicsConstraintComponent.SetAngularTwistLimit` _physicsconstraint "ACM_Locked" 0.0)
      (`PhysicsConstraintComponent.SetAngularSwing2Limit` _physicsconstraint "ACM_Locked" 0.0))))

(event `ResetTarget`
  ; Reset Cube Location
  (`self.ResetCube`))

(event `/Game/Production/Blueprints/Interfaces/BPI_TargetHit.HandleHit`
  (params (ScoreValue :type Integer))
  (bind _outactors (`GameplayStatics.GetAllActorsOfClass` "/Game/Production/Blueprints/BP_TargetManager.BP_TargetManager_C"))
  (`/Game/Production/Blueprints/BP_TargetManager.AddScore` (`|GetArrayItem` _outactors) 20))

(fn `ResetCube`
  (bind _physicsconstraint (`self.PhysicsConstraint`))
  (`PrimitiveComponent.SetSimulatePhysics` (`self.GravityCube`) false)
  (`SceneComponent.SetMobility` (`self.GravityCube`) "Movable")
  (`PrimitiveComponent.SetEnableGravity` (`self.GravityCube`) false)
  (`PhysicsConstraintComponent.SetLinearXLimit` _physicsconstraint "LCM_Free" 0.0)
  (`PhysicsConstraintComponent.SetLinearYLimit` _physicsconstraint "LCM_Free" 0.0)
  (`PhysicsConstraintComponent.SetLinearZLimit` _physicsconstraint "LCM_Free" 0.0)
  (`SceneComponent.K2_SetWorldTransform` (`self.GravityCube`) (`self.StartLocation`) false true)
  (`PrimitiveComponent.SetSimulatePhysics` (`self.GravityCube`) true)
  (`PrimitiveComponent.SetEnableGravity` (`self.GravityCube`) true)
  (set `self.CubeState` "NewEnumerator0"))

(fn `UserConstructionScript`)