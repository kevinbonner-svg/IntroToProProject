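; BP_Door is a level prop door that swings open and closed when interacted with, unless it is locked.
; DoorInteract calls Open or Close based on the Opened flag, which these graphs never set.
; A timeline drives the door's yaw through a lerp, playing forward to open and reversing to close.
; Unlock clears Locked before testing it, so its CallUnlocked branch never runs as written.
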(event `Open`
  ; Open and Close animations
  (if (not (`self.Locked`))
    (bind (_direction _doorrotation) (`Timeline|Timeline` :!label _label)
      (:`Update`
        (`SceneComponent.K2_SetRelativeRotation` (`self.Door`) (`KismetMathLibrary.MakeRotator` 0.0 0.0 (`KismetMathLibrary.Lerp` 0.0 110.0 _doorrotation)) false false)))))

(event `Close`
  ; Open and Close animations
  (if (not (`self.Locked`))
    (goto _label :!via `Reverse`)))

(event `Unlock`
  ; NOT SURE
  (set `self.Locked` false)
  (if (`self.Locked`)
    (`self.Unlocked`)))

(event `DoorInteract`
  (if (`self.Opened`)
    (`self.Close`)
    (else
      (`self.Open`))))

(fn `UserConstructionScript`)