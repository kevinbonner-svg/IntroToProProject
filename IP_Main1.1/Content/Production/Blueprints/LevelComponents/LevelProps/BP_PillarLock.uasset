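; BP_PillarLock is a level prop lock that unlocks once the player stays in its trigger long enough for the pillar to reach its unlock point.
; A timeline lerps the whole actor between two cached scene points, reversing if the player leaves early.
; Near the target it latches unlocked, swaps the pillar material and, given a valid UnlockManagerRef, registers the unlock and spawns Chase_AI enemies at random reachable points around itself.
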(event `self.TriggerBox.OnComponentBeginOverlap`
  (params (OverlappedComponent :type "PrimitiveComponent Object Reference") (OtherActor :type "Actor Object Reference") (OtherComp :type "PrimitiveComponent Object Reference") (OtherBodyIndex :type Integer) (bFromSweep :type Boolean) (SweepResult :type "HitResult Structure (by ref)"))
  (bind _unlockmanagerref (`self.UnlockManagerRef`))
  (cast `/Game/Production/Player/BP_Player` OtherActor)
  (if (not (`self.bIsUnlocked`))
    (bind (_direction _progress) (`Timeline|MoveTimeline` :!label _label)
      (:`Update`
        (`self.K2_SetActorLocation` (`KismetMathLibrary.VLerp` (`self.StartLocation`) (`self.UnlockLocation`) _progress))
        (if (<= (`KismetMathLibrary.VSize` (- (`self.K2_GetActorLocation`) (`self.UnlockLocation`))) 5.0)
          (if (not (`self.bIsUnlocked`))
            (set `self.bIsUnlocked` true)
            (`PrimitiveComponent.SetMaterial` (`self.PillarMesh`) 0 "/Game/Production/Meshes/Props/MM_HourGlass2.MM_HourGlass2")
            (`/Engine/EditorBlueprintResources/StandardMacros.IsValid` _unlockmanagerref
              (:`Is Valid`
                (if true
                  (`/Game/Production/Blueprints/BP_UnlockManager.RegisterUnlock` _unlockmanagerref)
                  (`self.Spawn Enemies`))))))))))

(event `self.TriggerBox.OnComponentEndOverlap`
  (params (OverlappedComponent :type "PrimitiveComponent Object Reference") (OtherActor :type "Actor Object Reference") (OtherComp :type "PrimitiveComponent Object Reference") (OtherBodyIndex :type Integer))
  (cast `/Game/Production/Player/BP_Player` OtherActor)
  (if (not (`self.bIsUnlocked`))
    (goto _label :!via `Reverse`)))

(event `Spawn Enemies`
  (for _ (range 6)
    (`|SpawnActorFromClass` "/Game/Production/AI/Enemies/Chase_AI.Chase_AI_C" (`KismetMathLibrary.Conv_VectorToTransform` (`NavigationSystemV1.K2_GetRandomReachablePointInRadius` (`SceneComponent.K2_GetComponentLocation` (`self.PillarMesh`)) 1000.0 null null)) "AdjustIfPossibleButAlwaysSpawn" "MultiplyWithRoot" null null)))

(event `self.ReceiveBeginPlay`
  (set `self.StartLocation` (`SceneComponent.K2_GetComponentLocation` (`self.StartPoint`)))
  (set `self.UnlockLocation` (`SceneComponent.K2_GetComponentLocation` (`self.UnlockPoint`))))

(fn `UserConstructionScript`)