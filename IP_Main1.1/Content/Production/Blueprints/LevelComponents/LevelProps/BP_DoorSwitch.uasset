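; BP_DoorSwitch is a level prop switch that opens and closes a referenced door when interacted with.
; Its Interact event prints a debug string, then uses a FlipFlop to alternate between two states on each use.
; One state lowers the button component slightly and calls Open on DoorRef, and the other raises it back and calls Close.
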(event `/Game/Production/Blueprints/Interfaces/BPI_Interact.Interact`
  (`KismetSystemLibrary.PrintString` "Interact Open Door")
  (`/Engine/EditorBlueprintResources/StandardMacros.FlipFlop`
    (:`A`
      (`SceneComponent.K2_SetWorldLocation` (`self.SwitchButton`) (- (`SceneComponent.K2_GetComponentLocation` (`self.SwitchButton`)) (0.0 0.0 4.0)) false false)
      (`/Game/Production/Blueprints/LevelComponents/LevelProps/BP_Door.Open` (`self.DoorRef`)))
    (:`B`
      (`SceneComponent.K2_SetWorldLocation` (`self.SwitchButton`) (+ (`SceneComponent.K2_GetComponentLocation` (`self.SwitchButton`)) (0.0 0.0 4.0)) false false)
      (`/Game/Production/Blueprints/LevelComponents/LevelProps/BP_Door.Close` (`self.DoorRef`)))))

(fn `UserConstructionScript`)