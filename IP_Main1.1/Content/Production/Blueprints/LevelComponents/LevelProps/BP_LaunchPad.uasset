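; BP_LaunchPad is a level prop that launches the player when they step onto it.
; Overlapping its Box casts to BP_Player and calls LaunchCharacter along the pad's forward and up vectors, scaled by ForwardVelocity and UpwardVelocity, overriding existing velocity.
; A RotatePad event turns the pad 90 degrees in yaw, changing the launch direction, and prints a debug string.
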(event `self.Box.OnComponentBeginOverlap`
  (params (OverlappedComponent :type "PrimitiveComponent Object Reference") (OtherActor :type "Actor Object Reference") (OtherComp :type "PrimitiveComponent Object Reference") (OtherBodyIndex :type Integer) (bFromSweep :type Boolean) (SweepResult :type "HitResult Structure (by ref)"))
  (bind _asbp_player (cast `/Game/Production/Player/BP_Player` OtherActor))
  (`Character.LaunchCharacter` _asbp_player (+ (* (`self.GetActorForwardVector`) (`self.ForwardVelocity`)) (* (`self.GetActorUpVector`) (`self.UpwardVelocity`))) true true))

(event `RotatePad`
  (`KismetSystemLibrary.PrintString` "Rotation Called")
  (`self.K2_SetActorRotation` (`KismetMathLibrary.MakeRotator` (.roll (`self.K2_GetActorRotation`)) (.pitch (`self.K2_GetActorRotation`)) (+ (.yaw (`self.K2_GetActorRotation`)) 90.0))))

(fn `UserConstructionScript`)