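; Hitscan weapon Blueprint that fires a rate-limited line trace from a supplied origin and direction.
; Shoot clears CanShoot and starts a FireDelay timer, with ShootTimerExpired re-enabling fire.
; It traces the Visibility channel over Range with debug drawing and a print.
; Movable, physics-simulating hits receive an impulse scaled by Damage, with no health damage applied, and are returned as a hit result.
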(event `ShootTimerExpired`
  (set `self.CanShoot` true))

(fn `Shoot`
  (params (OriginLocation :type "Vector Structure") (ForwardVector :type "Vector Structure"))
  (returns (HitEvent :type "HitResult Structure"))
  (if (`self.CanShoot`)
    (set `self.CanShoot` false)
    (`KismetSystemLibrary.K2_SetTimerDelegate` (`|CreateDelegate` :!event `ShootTimerExpired`) (`self.FireDelay`))
    (`KismetSystemLibrary.PrintString` "SHOOT")
    (bind _outhit (`KismetSystemLibrary.LineTraceSingle` :`Start` OriginLocation :`End` (+ OriginLocation (* ForwardVector (`self.Range`))) :`TraceChannel` "TraceTypeQuery1" :`DrawDebugType` "ForDuration"))
    (`/Engine/EditorBlueprintResources/StandardMacros.IsValid` (`.HitComponent` (`GameplayStatics.BreakHitResult` _outhit))
      (:`Is Valid`
        (if (and (`SceneComponent.IsSimulatingPhysics` (`.HitComponent` (`GameplayStatics.BreakHitResult` _outhit)) "None") (`|EnumEquality` (`SceneComponent.Mobility` (`.HitComponent` (`GameplayStatics.BreakHitResult` _outhit))) "Movable"))
          (`PrimitiveComponent.AddImpulseAtLocation` (`.HitComponent` (`GameplayStatics.BreakHitResult` _outhit)) (* ForwardVector (`self.Damage`)) (`.Location` (`GameplayStatics.BreakHitResult` _outhit)) "None")
          (return (`GameplayStatics.MakeHitResult` false false 0.0 0.0 (`.Location` (`GameplayStatics.BreakHitResult` _outhit)) (0.0 0.0 0.0) (0.0 0.0 1.0) (0.0 0.0 1.0) null (`.HitActor` (`GameplayStatics.BreakHitResult` _outhit)) (`.HitComponent` (`GameplayStatics.BreakHitResult` _outhit)))))))))

(fn `UserConstructionScript`)