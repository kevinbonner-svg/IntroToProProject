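; Shotgun weapon Blueprint that extends its parent's Shoot with a multi-pellet hitscan spread.
; Shoot calls the parent, then FireShotgun, which loops over PelletCount to trace on the Visibility channel along random directions within a SpreadAngle cone, out to ShotgunRange.
; Traces start at player 0's camera rather than using Shoot's origin and direction inputs.
; Traces only draw timed debug lines; their hit results are unused here.
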(event `FireShotgun`
  (bind _returnvalue (`self.GetComponentByClass` (`GameplayStatics.GetPlayerCharacter` 0) "/Script/Engine.CameraComponent"))
  (bind _returnvalue_2 (`SceneComponent.K2_GetComponentLocation` _returnvalue))
  (for _ (range (+ (`self.PelletCount`) 1))
    (`KismetSystemLibrary.LineTraceSingle` :`Start` _returnvalue_2 :`End` (+ _returnvalue_2 (* (`KismetMathLibrary.RandomUnitVectorInConeInDegrees` (`SceneComponent.GetForwardVector` _returnvalue) (`self.SpreadAngle`)) (`self.ShotgunRange`))) :`TraceChannel` "TraceTypeQuery1" :`DrawDebugType` "ForDuration")))

(fn `Shoot`
  (params (OriginLocation :type "Vector Structure") (ForwardVector :type "Vector Structure"))
  (returns (HitEvent :type "HitResult Structure"))
  (locals (NewLocalVar_0 :type "Vector Structure" :default (0.0 0.0 0.0)))
  (`parent.Shoot` OriginLocation ForwardVector)
  (`self.FireShotgun`)
  (return))

(fn `UserConstructionScript`
  (`parent.UserConstructionScript`))