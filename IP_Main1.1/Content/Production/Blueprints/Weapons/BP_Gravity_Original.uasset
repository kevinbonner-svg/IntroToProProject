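; BP_Gravity_Original is a weapon Blueprint that notifies cubes when they are shot.
; Its Shoot override calls the parent implementation with the origin and forward vector, then casts the returned hit actor to BP_Cube and calls OnShot on it.
; The hit detection comes from the parent class, and despite the name, no gravity logic appears in this Blueprint.
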(fn `Shoot`
  (params (OriginLocation :type "Vector Structure") (ForwardVector :type "Vector Structure"))
  (returns (HitEvent :type "HitResult Structure"))
  (locals (NewLocalVar :type "Actor Object Reference"))
  (bind _hitevent (`parent.Shoot` OriginLocation ForwardVector))
  (bind _asbp_cube (cast `/Game/Production/Blueprints/LevelComponents/LevelProps/BP_Cube` (`.HitActor` (`GameplayStatics.BreakHitResult` _hitevent))))
  (`/Game/Production/Blueprints/LevelComponents/LevelProps/BP_Cube.OnShot` _asbp_cube)
  (return))

(fn `UserConstructionScript`
  (`parent.UserConstructionScript`))