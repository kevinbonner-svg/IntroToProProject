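; BP_ObjectiveManager runs a sequence of objective actors in the order set by its OrderedObjectives array.
; On BeginPlay it hides every objective and activates the first; SetCurrentObjective unhides an objective, prints its instructions and binds an event to its completion.
; OnEventCompleted increments the index and activates that objective, calling itself recursively to skip invalid entries while the index is within the array length.
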(event `self.ReceiveBeginPlay`
  (if (`KismetArrayLibrary.Array_IsNotEmpty` (`self.OrderedObjectives`))
    (for _array_element (`self.OrderedObjectives`)
      (`self.SetActorHiddenInGame` _array_element true))
    (`self.SetCurrentObjective` (`|GetArrayItem` (`self.OrderedObjectives`)))))

(event `OnEventCompleted`
  ; Increase current index by one
  (bind _result (`/Engine/EditorBlueprintResources/StandardMacros.IncrementInt` (`self.CurrentObjectiveIndex`))
    (:`  `
      (bind _output (`|GetArrayItem` (`self.OrderedObjectives`) _result))
      ; Does this actor exist in level?
      (`/Engine/EditorBlueprintResources/StandardMacros.IsValid` _output
        (:`Is Valid`
          (`self.SetCurrentObjective` _output))
        (:`Is Not Valid`
          ; If this actor doesnt exist, skip to next index
          (if (< (`self.CurrentObjectiveIndex`) (`KismetArrayLibrary.Array_Length` (`self.OrderedObjectives`)))
            (`self.OnEventCompleted`)))))))

(fn `SetCurrentObjective`
  (params (NewObjective :type "/Game/Production/Blueprints/Objectives/BP_ObjectiveMarker Object Reference"))
  (`self.SetActorHiddenInGame` NewObjective false)
  (`KismetSystemLibrary.PrintString` (`/Game/Production/Blueprints/Objectives/BP_ObjectiveMarker.Instructions` NewObjective) true true (struct :`G` 0.66 :`B` 1.0 :`A` 1.0) 5.0)
  (add `/Game/Production/Blueprints/Objectives/BP_ObjectiveMarker.Completed` NewObjective (`|CreateDelegate` :!event `OnEventCompleted`)))

(fn `UserConstructionScript`)