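; BP_Gravity is a child Blueprint that overrides Shoot to make BP_Cube actors float.
; It calls the parent Shoot with an origin and forward vector, then casts the returned hit actor to BP_Cube.
; A hit cube has gravity disabled on its GravityCube component, starts its floating behavior and receives an upward velocity-change impulse, independent of mass.
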(fn `Shoot`
  (params (OriginLocation :type "Vector Structure") (ForwardVector :type "Vector Structure"))
  (returns (HitEvent :type "HitResult Structure"))
  (bind _hitevent (`parent.Shoot` OriginLocation ForwardVector))
  (bind _asbp_cube (cast `/Game/Production/Blueprints/LevelComponents/LevelProps/BP_Cube` (`.HitActor` (`GameplayStatics.BreakHitResult` _hitevent))))
  (bind _gravitycube (`/Game/Production/Blueprints/LevelComponents/LevelProps/BP_Cube.GravityCube` _asbp_cube))
  (`PrimitiveComponent.SetEnableGravity` _gravitycube false)
  (`/Game/Production/Blueprints/LevelComponents/LevelProps/BP_Cube.StartFLoating` _asbp_cube)
  (`PrimitiveComponent.AddImpulse` _gravitycube (0.0 0.0 500.0) "None" true)
  (return))

(fn `UserConstructionScript`
  (`parent.UserConstructionScript`))