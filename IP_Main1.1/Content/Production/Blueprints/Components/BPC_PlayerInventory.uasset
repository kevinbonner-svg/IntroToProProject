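; Player inventory component that tracks item quantities in a map keyed by item tag, with ammo among its apparent uses.
; AddItems stacks amounts onto existing entries or creates new ones, while GetItemCount and CanConsumeItem query the map.
; ConsumeItem subtracts only when enough is held, printing the count for debugging and a no-ammo message on failure.
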(fn `AddItems`
  (params (`Item Tag` :type "GameplayTag Structure") (Amount :type Integer))
  (locals (LocalAmount :type Integer) (LocalItemTag :type "GameplayTag Structure"))
  (set `local.LocalAmount` Amount)
  (set `local.LocalItemTag` `Item Tag`)
  (if (`BlueprintMapLibrary.Map_Contains` (`self.ItemQuantities`) (`local.LocalItemTag`))
    (`BlueprintMapLibrary.Map_Add` (`self.ItemQuantities`) (`local.LocalItemTag`) (+ (`BlueprintMapLibrary.Map_Find` (`self.ItemQuantities`) (`local.LocalItemTag`)) (`local.LocalAmount`)))
    (else
      (`BlueprintMapLibrary.Map_Add` (`self.ItemQuantities`) (`local.LocalItemTag`) (`local.LocalAmount`)))))

(fn `CanConsumeItem`
  (params (`Item Tag` :type "GameplayTag Structure") (Quantity :type Integer))
  (returns (CanConsume :type Boolean))
  (if (>= (`BlueprintMapLibrary.Map_Find` (`self.ItemQuantities`) `Item Tag`) Quantity)
    (return true)
    (else
      (return false))))

(fn `ConsumeItem`
  (params (`Item Tag` :type "GameplayTag Structure") (Amount :type Integer))
  (returns (Success :type Boolean))
  (locals (LocalAmount :type Integer) (LocalItemtag :type "GameplayTag Structure") (CurrentCount :type Integer :default 0))
  (set `local.LocalAmount` Amount)
  (set `local.LocalItemtag` `Item Tag`)
  (bind _count (`self.GetItemCount` (`local.LocalItemtag`)))
  (`KismetSystemLibrary.PrintString` (`KismetStringLibrary.Conv_IntToString` _count) true true (struct :`R` 1.0 :`B` 0.04737 :`A` 1.0) 5.0)
  (set `local.CurrentCount` _count)
  (if (>= _count (`local.LocalAmount`))
    (`BlueprintMapLibrary.Map_Add` (`self.ItemQuantities`) (`local.LocalItemtag`) (- (`local.CurrentCount`) (`local.LocalAmount`)))
    (return true)
    (else
      (`KismetSystemLibrary.PrintString` "NO AMMO CANT SHOOT"))))

(fn `GetItemCount`
  (params (ItemTag :type "GameplayTag Structure"))
  (returns (Count :type Integer))
  (return (`BlueprintMapLibrary.Map_Find` (`self.ItemQuantities`) ItemTag)))