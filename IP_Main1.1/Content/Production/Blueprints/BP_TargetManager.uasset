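; BP_TargetManager tracks a total score and manages resets for the two kinds of target in the level.
; On BeginPlay it gathers all BP_Cube and BP_CubeTarget actors into two separate lists.
; AddScore adds to the running total, and separate events zero the score or loop through each list calling that target type's reset.
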(event `ResetScore`
  (set `self.TotalScore` 0))

(event `ResetBPCubeTargets`
  (for _array_element (`self.BPCubeTargets`)
    (`/Game/Production/Blueprints/LevelComponents/BP_CubeTarget.ResetTargetCube` _array_element)))

(event `ResetAllTargets`
  (for _array_element (`self.TargetList`)
    (`/Game/Production/Blueprints/LevelComponents/LevelProps/BP_Cube.ResetTarget` _array_element)))

(event `self.ReceiveBeginPlay`
  (`|ExecutionSequence`
    (:`then_0`
      (bind _outactors (`GameplayStatics.GetAllActorsOfClass` "/Game/Production/Blueprints/LevelComponents/LevelProps/BP_Cube.BP_Cube_C"))
      (set `self.TargetList` _outactors))
    (:`then_1`
      (bind _outactors_2 (`GameplayStatics.GetAllActorsOfClass` "/Game/Production/Blueprints/LevelComponents/BP_CubeTarget.BP_CubeTarget_C"))
      (set `self.BPCubeTargets` _outactors_2))))

(fn `AddScore`
  (params (ScoreToAdd :type Integer))
  (set `self.TotalScore` (+ ScoreToAdd (`self.TotalScore`))))

(fn `UserConstructionScript`)