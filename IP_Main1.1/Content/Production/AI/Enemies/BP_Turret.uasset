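; Enemy turret that aims and fires at the player when its PawnSensing component sees them, and is destroyed when its health component is depleted.
; Each sighting runs TargetPlayer, which interpolates toward a look-at rotation, turning the whole actor for yaw and tilting only the Head for clamped pitch.
; It then calls Shoot on the BP_TurretGun child actor cached at BeginPlay, using BulletStart's location and forward vector.
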(event `self.ReceiveBeginPlay`
  (bind _asbp_turret_gun (cast `/Game/Production/Blueprints/Weapons/BP_TurretGun` (`ChildActorComponent.ChildActor` (`self.Gun`))))
  (set `self.GunBP` _asbp_turret_gun))

(event `self.PawnSensing.OnSeePawn`
  (params (Pawn :type "Pawn Object Reference"))
  (bind _bulletstart (`self.BulletStart`))
  (bind _asbp_player (cast `/Game/Production/Player/BP_Player` Pawn))
  (`self.TargetPlayer` _asbp_player)
  (`/Game/Production/Blueprints/BP_Weapon.Shoot` (`self.GunBP`) (`SceneComponent.K2_GetComponentLocation` _bulletstart) (`SceneComponent.GetForwardVector` _bulletstart)))

(event `self.BPC_Health.OnHealthDepleted`
  (`self.K2_DestroyActor`))

(fn `TargetPlayer`
  (params (player :type "Actor Object Reference"))
  (bind _head (`self.Head`))
  (bind (_returnvalue_roll _returnvalue_pitch _returnvalue_yaw) (`KismetMathLibrary.BreakRotator` (`KismetMathLibrary.RInterpTo` (`SceneComponent.K2_GetComponentRotation` _head) (`KismetMathLibrary.FindLookAtRotation` (`SceneComponent.K2_GetComponentLocation` _head) (`self.K2_GetActorLocation` player)) (`GameplayStatics.GetWorldDeltaSeconds`) 15.0)))
  (`SceneComponent.K2_SetRelativeRotation` (`self.Head`) (`KismetMathLibrary.MakeRotator` 0.0 (`KismetMathLibrary.FClamp` _returnvalue_pitch -20.0 20.0)) false false)
  (`self.K2_SetActorRotation` (`KismetMathLibrary.MakeRotator` 0.0 0.0 _returnvalue_yaw)))

(fn `UserConstructionScript`)